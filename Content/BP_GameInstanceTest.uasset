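; BP_GameInstanceTest, by its name a test Game Instance, provides helper functions for playing sounds and opening levels.
; Sound keys index a SoundCollection map, and the result plays either in 2D or at a given location, with a debug print of the key.
; Level keys index a LevelsName map to open the matching level by name, and no lookup checks whether the key was found.
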(fn FPlaySound2d
  (params (Sound :type E_SoundNames%20Enum :default "NewEnumerator2"))
  (Audio|PlaySound2D (.Value (Utilities|Map|Find (Variables|Default|GetSoundCollection) Sound)) 1.0 1.0 0.0 0 0)
  (Development|PrintString (Utilities|String|Append "Play sound: " (Utilities|String|EnumtoString Sound))))

(fn FPlaySoundatLocation
  (params (Sound :type E_SoundNames%20Enum :default "NewEnumerator2") (Location :type Vector))
  (Audio|PlaySoundatLocation (.Value (Utilities|Map|Find (Variables|Default|GetSoundCollection) Sound)) Location "0, 0, 0" 1.0 1.0 0.0 0 0 0 0)
  (Development|PrintString (Utilities|String|Append "Play sound: " (Utilities|String|EnumtoString Sound))))

(fn FOpenLevel
  (params (Level :type E_LevelsName%20Enum :default "NewEnumerator2"))
  (Game|OpenLevel(byName) (.Value (Utilities|Map|Find (Variables|Default|GetLevelsName) Level))))