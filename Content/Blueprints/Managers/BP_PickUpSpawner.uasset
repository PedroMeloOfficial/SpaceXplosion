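; Manager actor that spawns repair pickups (BP_RepairPickUp) at random points around the player throughout play.
; BeginPlay caches the BP_Player reference and spawns a first pickup inside the bounds of the player's PickUpSpawner component.
; Tick repeats that spawn through a DoOnce that a Delay resets, giving a timed spawn loop without a timer.
; Spawns adjust for collision but always succeed.
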(event EventBeginPlay
  (bind _asbp_player (Utilities|Casting|CastToBP_Player (Game|GetPlayerCharacter 0)))
  (bind _output_get (Variables|Default|SetAs%20BP%20Player _asbp_player))
  (for _index (range 1 1)
    (Game|SpawnActorfromClass "/Game/Blueprints/GameplayObjects/BP_RepairPickUp.BP_RepairPickUp_C" (Math|Transform|MakeTransform (Math|Random|RandomPointinBoundingBox (.Origin (Collision|GetComponentBounds (Variables|/Game/Blueprints/Character/BP_Player.BP_Player_C|GetPickUpSpawner _output_get))) (.BoxExtent (Collision|GetComponentBounds (Variables|/Game/Blueprints/Character/BP_Player.BP_Player_C|GetPickUpSpawner _output_get)))) "0, 0, 0" "1.000000,1.000000,1.000000") "AdjustIfPossibleButAlwaysSpawn" "MultiplyWithRoot" 0 0)))

(event EventTick
  (params (DeltaSeconds :type Float%20%28single-precision%29))
  (bind _as_bp_player (Variables|Default|GetAs%20BP%20Player))
  (bind _pickupspawner (Variables|/Game/Blueprints/Character/BP_Player.BP_Player_C|GetPickUpSpawner _as_bp_player))
  (bind (_origin _boxextent) (Collision|GetComponentBounds _pickupspawner))
  (Utilities|FlowControl|DoOnce false :!label _label
    (:Completed
      (Game|SpawnActorfromClass "/Game/Blueprints/GameplayObjects/BP_RepairPickUp.BP_RepairPickUp_C" (Math|Transform|MakeTransform (Math|Random|RandomPointinBoundingBox _origin _boxextent) "0, 0, 0" "1.000000,1.000000,1.000000") "AdjustIfPossibleButAlwaysSpawn" "MultiplyWithRoot" 0 0)
      (Utilities|FlowControl|Delay 6.0)
      (goto _label Reset))))

(fn ConstructionScript)