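; Spawner actor that fills a box volume with asteroids and keeps spawning moving ones during play.
; On BeginPlay it spawns a starting batch of BP_Asteroid at random points in the box, each given an emissive material.
; A Tick-driven DoOnce, reset after a delay, repeatedly spawns an emissive BP_AsteroidMov in the box.
; Each moving asteroid is oriented along the direction from the spawner to the player's current location.
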(event EventBeginPlay
  (bind _box (Variables|Default|GetBox))
  (bind _box_2 (Variables|Default|GetBox))
  (bind (_origin _boxextent) (Collision|GetComponentBounds _box_2))
  (bind (_origin_2 _boxextent_2) (Collision|GetComponentBounds _box))
  (bind _asbp_player (Utilities|Casting|CastToBP_Player (Game|GetPlayerCharacter 0)))
  (Variables|Default|SetAs%20BP%20Player _asbp_player)
  (for _index (range 1 (Variables|Default|GetAsteroidsSpawnBegin))
    (bind _returnvalue (Game|SpawnActorfromClass "/Game/Blueprints/GameplayObjects/BP_Asteroid.BP_Asteroid_C" (Math|Transform|MakeTransform (Math|Random|RandomPointinBoundingBox _origin _boxextent) "0, 0, 0" "1.000000,1.000000,1.000000") "AdjustIfPossibleButAlwaysSpawn" "MultiplyWithRoot" 0 0))
    (Rendering|Material|SetMaterial (Variables|/Game/Blueprints/GameplayObjects/BP_Asteroid.BP_Asteroid_C|GetAsteroidMesh _returnvalue) 0 "/Game/Assets/Shaders/M_Emissive.M_Emissive"))
  (Utilities|FlowControl|DoOnce true) ; enters at Reset
)

(event EventTick
  (params (DeltaSeconds :type Float%20%28single-precision%29))
  (bind _box (Variables|Default|GetBox))
  (bind (_origin _boxextent) (Collision|GetComponentBounds _box))
  (Utilities|FlowControl|DoOnce true :!label _label
    (:Completed
      (bind _returnvalue (Game|SpawnActorfromClass "/Game/Blueprints/GameplayObjects/BP_AsteroidMov.BP_AsteroidMov_C" (Math|Transform|MakeTransform (Math|Random|RandomPointinBoundingBox _origin _boxextent) (Math|Conversions|RotationFromXVector (- (Transformation|GetActorLocation (Variables|Default|GetAs%20BP%20Player)) (Transformation|GetActorLocation))) "1.000000,1.000000,1.000000") "AdjustIfPossibleButAlwaysSpawn" "MultiplyWithRoot" 0 0))
      (Rendering|Material|SetMaterial (Variables|/Game/Blueprints/GameplayObjects/BP_AsteroidMov.BP_AsteroidMov_C|GetAsteroidMesh _returnvalue) 0 "/Game/Assets/Shaders/M_Emissive.M_Emissive")
      (Utilities|FlowControl|Delay (Variables|Default|GetAsteroidSpawnDelay))
      (goto _label Reset))))

(fn ConstructionScript)