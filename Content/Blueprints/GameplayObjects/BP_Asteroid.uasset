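; Asteroid actor that takes a random mesh, scale and mass on spawn and reacts to collisions.
; Mesh scale, mass and radial force scale are each randomized separately.
; A hit fires a radial impulse and debris particles, throttled by a DoOnce that resets after a short delay.
; The crash sound's inverted OR of two inequality checks requires OtherActor to equal both asteroid references at once.
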(event OnComponentHit(AsteroidMesh)
  (params (HitComponent :type Primitive%20Component%20Object%20Reference) (OtherActor :type Actor%20Object%20Reference) (OtherComp :type Primitive%20Component%20Object%20Reference) (NormalImpulse :type Vector :default "0, 0, 0") (Hit :type Hit%20Result%20Structure%20%28by%20ref%29))
  (bind _location (Collision|BreakHitResult Hit))
  (Utilities|FlowControl|DoOnce false :!label _label
    (:Completed
      (Development|PrintString "Asteroid Hit" true true "(R=0.109733,G=1.000000,B=0.000000,A=1.000000)" 5.0)
      (Class|RadialForceComponent|FireImpulse (Variables|Default|GetRadialForce))
      (Effects|SpawnEmitteratLocation "/Game/Realistic_Starter_VFX_Pack_Vol2/Particles/Destruction/P_Destruction_Concrete.P_Destruction_Concrete" _location "0, 0, 0" "0.500000,0.500000,0.500000")
      (if (or (!= OtherActor "BP_Asteroid") (!= OtherActor "/Game/Blueprints/GameplayObjects/BP_AsteroidMov.BP_AsteroidMov"))
        _
        (else
          (Audio|PlaySoundatLocation "/Game/Assets/Sounds/crash-7075.crash-7075" _location "0, 0, 0" 0.9 0.9 0.0 0 0 0 0)))
      (Utilities|FlowControl|Delay 0.25)
      (goto _label Reset))))

(event EventBeginPlay
  (bind _returnvalue (Math|Random|RandomFloatinRange 0.4 1.2))
  (bind _asteroidmesh (Variables|Default|GetAsteroidMesh))
  (bind _returnvalue_2 (Math|Conversions|ToVector(Float) _returnvalue))
  (Components|StaticMesh|SetStaticMesh (Variables|Default|GetAsteroidMesh) (.OutItem (Utilities|Array|Random (Variables|Default|GetAsteroidMeshes))))
  (Transformation|SetWorldScale3D _asteroidmesh _returnvalue_2)
  (Class|PrimitiveComponent|SetMassOverrideinKg _asteroidmesh "None" (* _returnvalue 1e+03) true)
  (Transformation|SetWorldScale3D (Variables|Default|GetRadialForce) _returnvalue_2))

(event EventTick
  (params (DeltaSeconds :type Float%20%28single-precision%29)))

(fn ConstructionScript)