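; BP_RepairPickUp is a repair pickup that heals the player on contact.
; On begin play it caches the player character as BP_Player, then turns every tick to face that player.
; When a BP_Player overlaps its box collider, it applies its heal amount through FTakeHeal, plays a beep and destroys itself.
; A health check on the player is left unconnected, so healing happens regardless of current health.
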(event OnComponentBeginOverlap(BoxCollider)
  (params (OverlappedComponent :type Primitive%20Component%20Object%20Reference) (OtherActor :type Actor%20Object%20Reference) (OtherComp :type Primitive%20Component%20Object%20Reference) (OtherBodyIndex :type Integer) (bFromSweep :type Boolean) (SweepResult :type Hit%20Result%20Structure%20%28by%20ref%29))
  (bind _asbp_player (Utilities|Casting|CastToBP_Player OtherActor))
  (Default|FTakeHeal _asbp_player (Variables|Default|GetHealAmount))
  (Audio|PlaySoundatLocation "/Game/Assets/Sounds/one_beep-99630.one_beep-99630" (Transformation|GetWorldLocation (Variables|Default|GetBoxCollider)) "0, 0, 0" 1.0 1.0 0.0 0 0 0 0)
  (Actor|DestroyActor))

(event EventBeginPlay
  (bind _asbp_player (Utilities|Casting|CastToBP_Player (Game|GetPlayerCharacter 0)))
  (Variables|Default|SetAs%20BP%20Player _asbp_player))

(event EventTick
  (params (DeltaSeconds :type Float%20%28single-precision%29))
  (Transformation|SetActorRotation (CallFunction|PCalcRottoFacePlayer)))

(fn ConstructionScript)

(fn PCalcRottoFacePlayer
  (return (Math|Conversions|RotationFromXVector (Math|Vector|RotateVector (- (Transformation|GetActorLocation (Variables|Default|GetAs%20BP%20Player)) (Transformation|GetActorLocation)) "0, 0, 0"))))