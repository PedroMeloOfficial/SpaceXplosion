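; BP_ISS is a breakable ISS space station whose parts come loose when hit by a laser blast or the player.
; Parts 2, 3 and 4 each handle their own hit event, accepting only BP_LaserBlast or BP_Player.
; A valid hit applies a radial impulse at the impact point, then enables physics on that part and plays a crash sound there.
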(event OnComponentHit(ISS_part2)
  (params (HitComponent :type Primitive%20Component%20Object%20Reference) (OtherActor :type Actor%20Object%20Reference) (OtherComp :type Primitive%20Component%20Object%20Reference) (NormalImpulse :type Vector :default "0, 0, 0") (Hit :type Hit%20Result%20Structure%20%28by%20ref%29))
  (bind _location (Collision|BreakHitResult Hit))
  (Utilities|FlowControl|Sequence
    (:then_0
      (Utilities|Casting|CastToBP_LaserBlast OtherActor))
    (:then_1
      (Utilities|Casting|CastToBP_Player OtherActor)))
  (Physics|AddRadialImpulse (Variables|Default|GetISS_part2) _location 3e+02 3e+04 "RIF_Constant" false)
  (Physics|SetSimulatePhysics (Variables|Default|GetISS_part2) true)
  (Audio|PlaySoundatLocation "/Game/Assets/Sounds/crash-7075.crash-7075" _location "0, 0, 0" 1.0 1.0 0.0 0 0 0 0))

(event OnComponentHit(ISS_part4)
  (params (HitComponent :type Primitive%20Component%20Object%20Reference) (OtherActor :type Actor%20Object%20Reference) (OtherComp :type Primitive%20Component%20Object%20Reference) (NormalImpulse :type Vector :default "0, 0, 0") (Hit :type Hit%20Result%20Structure%20%28by%20ref%29))
  (bind _location (Collision|BreakHitResult Hit))
  (Utilities|FlowControl|Sequence
    (:then_0
      (Utilities|Casting|CastToBP_LaserBlast OtherActor))
    (:then_1
      (Utilities|Casting|CastToBP_Player OtherActor)))
  (Physics|AddRadialImpulse (Variables|Default|GetISS_part4) _location 3e+02 3e+04 "RIF_Constant" false)
  (Physics|SetSimulatePhysics (Variables|Default|GetISS_part4) true)
  (Audio|PlaySoundatLocation "/Game/Assets/Sounds/crash-7075.crash-7075" _location "0, 0, 0" 1.0 1.0 0.0 0 0 0 0))

(event OnComponentHit(ISS_part3)
  (params (HitComponent :type Primitive%20Component%20Object%20Reference) (OtherActor :type Actor%20Object%20Reference) (OtherComp :type Primitive%20Component%20Object%20Reference) (NormalImpulse :type Vector :default "0, 0, 0") (Hit :type Hit%20Result%20Structure%20%28by%20ref%29))
  (bind _location (Collision|BreakHitResult Hit))
  (Utilities|FlowControl|Sequence
    (:then_0
      (Utilities|Casting|CastToBP_LaserBlast OtherActor))
    (:then_1
      (Utilities|Casting|CastToBP_Player OtherActor)))
  (Physics|AddRadialImpulse (Variables|Default|GetISS_part3) _location 3e+02 3e+04 "RIF_Constant" false)
  (Physics|SetSimulatePhysics (Variables|Default|GetISS_part3) true)
  (Audio|PlaySoundatLocation "/Game/Assets/Sounds/crash-7075.crash-7075" _location "0, 0, 0" 1.0 1.0 0.0 0 0 0 0))

(event EventBeginPlay)

(event EventTick
  (params (DeltaSeconds :type Float%20%28single-precision%29)))

(fn ConstructionScript)