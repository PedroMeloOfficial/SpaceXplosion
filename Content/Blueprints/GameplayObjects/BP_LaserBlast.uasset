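; BP_LaserBlast is a laser shot actor that explodes on impact.
; On BeginPlay it caches BP_GameInstanceTest and plays a spawn sound through it.
; When its Box component hits something, it fires a RadialForce impulse, spawns an explosion emitter and sound at the hit point, then destroys itself.
; Unconnected nodes for an electric emitter following the player's LaserSpawn point never run, and a debug print remains on hit.
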(event OnComponentHit(Box)
  (params (HitComponent :type Primitive%20Component%20Object%20Reference) (OtherActor :type Actor%20Object%20Reference) (OtherComp :type Primitive%20Component%20Object%20Reference) (NormalImpulse :type Vector :default "0, 0, 0") (Hit :type Hit%20Result%20Structure%20%28by%20ref%29))
  (bind _location (Collision|BreakHitResult Hit))
  (Development|PrintString "Laser Hit" true true "(R=0.071203,G=1.000000,B=0.000000,A=1.000000)" 5.0)
  (Class|RadialForceComponent|FireImpulse (Variables|Default|GetRadialForce))
  (Effects|SpawnEmitteratLocation "/Game/StarterContent/Particles/P_Explosion.P_Explosion" _location)
  (Default|FPlaySoundatLocation (Variables|Default|GetGIRef) "NewEnumerator6" _location)
  (Actor|DestroyActor))

(event EventBeginPlay
  (bind _asbp_game_instance_test (Utilities|Casting|CastToBP_GameInstanceTest (Game|GetGameInstance)))
  (bind _output_get (Variables|Default|SetGIRef _asbp_game_instance_test))
  (Default|FPlaySoundatLocation _output_get "NewEnumerator7" (Transformation|GetActorLocation)))

(event EventTick
  (params (DeltaSeconds :type Float%20%28single-precision%29)))

(fn ConstructionScript)