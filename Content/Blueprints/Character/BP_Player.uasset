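; Player astronaut pawn for space flight, with laser shooting, health, boost and a pause menu.
; Enhanced Input drives thruster components for movement, look and roll, while boost raises main thrust from a regenerating reserve.
; Tick projects a laser-aligned trace to a crosshair screen position and feeds smoothed motion deltas into a parallax Material Parameter Collection.
; Collisions deal damage and apply impulses; ammo reloads manually or when empty.
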(event OnComponentHit(CapsuleComponent)
  (params (HitComponent :type Primitive%20Component%20Object%20Reference) (OtherActor :type Actor%20Object%20Reference) (OtherComp :type Primitive%20Component%20Object%20Reference) (NormalImpulse :type Vector :default "0, 0, 0") (Hit :type Hit%20Result%20Structure%20%28by%20ref%29))
  (CallFunction|FTakeDamage 1)
  (Physics|AddImpulse (Variables|Collision|GetCapsuleComponent) NormalImpulse "None" false)
  (Audio|PlaySoundatLocation "/Game/Assets/Sounds/crash-7075.crash-7075" NormalImpulse "0, 0, 0" 1.0 1.0 0.0 0 0 0 0))

(event OnComponentHit(Cube1)
  (params (HitComponent :type Primitive%20Component%20Object%20Reference) (OtherActor :type Actor%20Object%20Reference) (OtherComp :type Primitive%20Component%20Object%20Reference) (NormalImpulse :type Vector :default "0, 0, 0") (Hit :type Hit%20Result%20Structure%20%28by%20ref%29))
  (CallFunction|FTakeDamage 1)
  (Physics|AddImpulse (Variables|Collision|GetCapsuleComponent) NormalImpulse "None" false)
  (Audio|PlaySoundatLocation "/Game/Assets/Sounds/crash-7075.crash-7075" NormalImpulse "0, 0, 0" 1.0 1.0 0.0 0 0 0 0))

(event OnComponentHit(Cube2)
  (params (HitComponent :type Primitive%20Component%20Object%20Reference) (OtherActor :type Actor%20Object%20Reference) (OtherComp :type Primitive%20Component%20Object%20Reference) (NormalImpulse :type Vector :default "0, 0, 0") (Hit :type Hit%20Result%20Structure%20%28by%20ref%29))
  (CallFunction|FTakeDamage 1)
  (Physics|AddImpulse (Variables|Collision|GetCapsuleComponent) NormalImpulse "None" false)
  (Audio|PlaySoundatLocation "/Game/Assets/Sounds/crash-7075.crash-7075" NormalImpulse "0, 0, 0" 1.0 1.0 0.0 0 0 0 0))

(event Input|EnhancedActionEvents|EnhancedInputActionIA_Move-Up
  (params (ActionValue :type Float%20%28double-precision%29) (ElapsedSeconds :type Float%20%28double-precision%29) (TriggeredSeconds :type Float%20%28double-precision%29) (InputAction :type Input%20Action%20Object%20Reference :default "/Game/Inputs/Actions/IA_Move-Up.IA_Move-Up"))
  (bind _thruster_up (Variables|Default|GetThruster_Up))
  ;[1 0.2592 0 0.5] INPUTACTION: Set thurster to active and set thurster strength
  (:Triggered
    (Components|Activation|SetActive _thruster_up true false :!label _label)
    (Variables|/Script/Engine.PhysicsThrusterComponent|SetThrustStrength _thruster_up (* ActionValue (Variables|Default|GetThrusterPowerMain))))
  (:Canceled
    (goto _label))
  (:Completed
    (goto _label)))

(event Input|EnhancedActionEvents|EnhancedInputActionIA_Move-Down
  (params (ActionValue :type Float%20%28double-precision%29) (ElapsedSeconds :type Float%20%28double-precision%29) (TriggeredSeconds :type Float%20%28double-precision%29) (InputAction :type Input%20Action%20Object%20Reference :default "/Game/Inputs/Actions/IA_Move-Down.IA_Move-Down"))
  (bind _thruster_down (Variables|Default|GetThruster_Down))
  ;[1 0.302 0] INPUTACTION: Set thurster to active and set thurster strength
  (:Triggered
    (Components|Activation|SetActive _thruster_down true false :!label _label)
    (Variables|/Script/Engine.PhysicsThrusterComponent|SetThrustStrength _thruster_down (* ActionValue (Variables|Default|GetThrusterPowerMain))))
  (:Canceled
    (goto _label))
  (:Completed
    (goto _label)))

(event Input|EnhancedActionEvents|EnhancedInputActionIA_Boost
  (params (ActionValue :type Boolean) (ElapsedSeconds :type Float%20%28double-precision%29) (TriggeredSeconds :type Float%20%28double-precision%29) (InputAction :type Input%20Action%20Object%20Reference :default "/Game/Inputs/Actions/IA_Boost.IA_Boost"))
  ;[1 0.3233 0 0.5] INPUTACTION: When trigger sets thurster strength to boost power, when canceled sets thurster strength to normal power
  (:Triggered
    (if (> (Variables|Default|GetCurrentBoost) 0.0)
      (Variables|Default|SetThrusterPowerMain (Variables|Default|GetBoostPower))
      (Variables|Default|SetCurrentBoost (Math|Float|Clamp(Float) (- (Variables|Default|GetCurrentBoost) 0.005) 0.0 (Variables|Default|GetMaxBoost)))))
  (:Canceled
    (Variables|Default|SetThrusterPowerMain (Variables|Default|GetNormalPower) :!label _label))
  (:Completed
    (goto _label)))

(event Input|EnhancedActionEvents|EnhancedInputActionIA_Reload
  (params (ActionValue :type Boolean) (ElapsedSeconds :type Float%20%28double-precision%29) (TriggeredSeconds :type Float%20%28double-precision%29) (InputAction :type Input%20Action%20Object%20Reference :default "/Game/Inputs/Actions/IA_Reload.IA_Reload"))
  (:Started
    (if (Variables|Default|GetCanShoot)
      (CallFunction|FReloadAmmo)
      (Utilities|FlowControl|Delay (Variables|Default|GetReloadDelay))
      (Variables|Default|SetCanShoot true))))

(event Input|EnhancedActionEvents|EnhancedInputActionIA_OpenMenu
  (params (ActionValue :type Boolean) (ElapsedSeconds :type Float%20%28double-precision%29) (TriggeredSeconds :type Float%20%28double-precision%29) (InputAction :type Input%20Action%20Object%20Reference :default "/Game/Inputs/Actions/IA_OpenMenu.IA_OpenMenu"))
  (:Started
    (bind _returnvalue (UserInterface|CreateWidget "/Game/UI/WBP_PauseMenu.WBP_PauseMenu_C"))
    (bind _output_get (Variables|Default|SetPauseMenuWidget _returnvalue))
    (UserInterface|Viewport|AddtoViewport _output_get 0)
    (Game|SetGamePaused true)))

(event Input|EnhancedActionEvents|EnhancedInputActionIA_Look
  (params (ActionValue :type Vector%202D%20Structure) (ElapsedSeconds :type Float%20%28double-precision%29) (TriggeredSeconds :type Float%20%28double-precision%29) (InputAction :type Input%20Action%20Object%20Reference :default "/Game/Inputs/Actions/IA_Look.IA_Look"))
  (bind (_x _y) (Math|Vector2D|BreakVector2D ActionValue))
  (bind _thruster_pitchleft (Variables|Default|GetThruster_PitchLeft))
  (bind _thruster_pitchright (Variables|Default|GetThruster_PitchRight))
  (bind _thruster_pitchforward (Variables|Default|GetThruster_PitchForward))
  (bind _thruster_pitchbackward (Variables|Default|GetThruster_PitchBackward))
  (bind _camerasensibility (Variables|Default|GetCameraSensibility))
  (bind _returnvalue (* _y _camerasensibility))
  (bind _returnvalue_2 (* _x _camerasensibility))
  ;[1 0.286 0 0.5] INPUTACTION: Set thurster to active and set thurster strength
  (:Triggered
    (Components|Activation|SetActive _thruster_pitchleft true false :!label _label)
    (Variables|/Script/Engine.PhysicsThrusterComponent|SetThrustStrength _thruster_pitchleft (* (* _returnvalue_2 (Variables|Default|GetThrusterPower)) -1.0))
    (Components|Activation|SetActive _thruster_pitchright true false)
    (Variables|/Script/Engine.PhysicsThrusterComponent|SetThrustStrength _thruster_pitchright (* (* _returnvalue_2 (Variables|Default|GetThrusterPower)) -1.0))
    (Components|Activation|SetActive _thruster_pitchforward true false)
    (Variables|/Script/Engine.PhysicsThrusterComponent|SetThrustStrength _thruster_pitchforward (* (* _returnvalue (Variables|Default|GetThrusterPower)) -1.0))
    (Components|Activation|SetActive _thruster_pitchbackward true false)
    (Variables|/Script/Engine.PhysicsThrusterComponent|SetThrustStrength _thruster_pitchbackward (* (* _returnvalue (Variables|Default|GetThrusterPower)) -1.0)))
  (:Canceled
    (goto _label))
  (:Completed
    (goto _label)))

(event Input|EnhancedActionEvents|EnhancedInputActionIA_Move-Forward
  (params (ActionValue :type Float%20%28double-precision%29) (ElapsedSeconds :type Float%20%28double-precision%29) (TriggeredSeconds :type Float%20%28double-precision%29) (InputAction :type Input%20Action%20Object%20Reference :default "/Game/Inputs/Actions/IA_Move-Forward.IA_Move-Forward"))
  (bind _thruster_forward (Variables|Default|GetThruster_Forward))
  ;[1 0.3325 0 0.5] INPUTACTION: Set thurster to active and set thurster strength
  (:Triggered
    (Components|Activation|SetActive _thruster_forward true false :!label _label)
    (Variables|/Script/Engine.PhysicsThrusterComponent|SetThrustStrength _thruster_forward (* ActionValue (Variables|Default|GetThrusterPowerMain))))
  (:Canceled
    (goto _label))
  (:Completed
    (goto _label)))

(event Input|EnhancedActionEvents|EnhancedInputActionIA_Move-Backward
  (params (ActionValue :type Float%20%28double-precision%29) (ElapsedSeconds :type Float%20%28double-precision%29) (TriggeredSeconds :type Float%20%28double-precision%29) (InputAction :type Input%20Action%20Object%20Reference :default "/Game/Inputs/Actions/IA_Move-Backward.IA_Move-Backward"))
  (bind _thruster_backward (Variables|Default|GetThruster_Backward))
  ;[1 0.3692 0 0.5] INPUTACTION: Set thurster to active and set thurster strength
  (:Triggered
    (Components|Activation|SetActive _thruster_backward true false :!label _label)
    (Variables|/Script/Engine.PhysicsThrusterComponent|SetThrustStrength _thruster_backward (* ActionValue (Variables|Default|GetThrusterPowerMain))))
  (:Canceled
    (goto _label))
  (:Completed
    (goto _label)))

(event Input|EnhancedActionEvents|EnhancedInputActionIA_Move_Left
  (params (ActionValue :type Float%20%28double-precision%29) (ElapsedSeconds :type Float%20%28double-precision%29) (TriggeredSeconds :type Float%20%28double-precision%29) (InputAction :type Input%20Action%20Object%20Reference :default "/Game/Inputs/Actions/IA_Move_Left.IA_Move_Left"))
  (bind _thruster_right (Variables|Default|GetThruster_Right))
  ;[1 0.3487 0 0.5] INPUTACTION: Set thurster to active and set thurster strength
  (:Triggered
    (Components|Activation|SetActive _thruster_right true false :!label _label)
    (Variables|/Script/Engine.PhysicsThrusterComponent|SetThrustStrength _thruster_right (* ActionValue (Variables|Default|GetThrusterPowerMain))))
  (:Canceled
    (goto _label))
  (:Completed
    (goto _label)))

(event Input|EnhancedActionEvents|EnhancedInputActionIA_Move_Right
  (params (ActionValue :type Float%20%28double-precision%29) (ElapsedSeconds :type Float%20%28double-precision%29) (TriggeredSeconds :type Float%20%28double-precision%29) (InputAction :type Input%20Action%20Object%20Reference :default "/Game/Inputs/Actions/IA_Move_Right.IA_Move_Right"))
  (bind _thruster_left (Variables|Default|GetThruster_Left))
  ;[1 0.3748 0 0.5] INPUTACTION: Set thurster to active and set thurster strength
  (:Triggered
    (Components|Activation|SetActive _thruster_left true false :!label _label)
    (Variables|/Script/Engine.PhysicsThrusterComponent|SetThrustStrength _thruster_left (* ActionValue (Variables|Default|GetThrusterPowerMain))))
  (:Canceled
    (goto _label))
  (:Completed
    (goto _label)))

(event Input|EnhancedActionEvents|EnhancedInputActionIA_Move-RollRight
  (params (ActionValue :type Float%20%28double-precision%29) (ElapsedSeconds :type Float%20%28double-precision%29) (TriggeredSeconds :type Float%20%28double-precision%29) (InputAction :type Input%20Action%20Object%20Reference :default "/Game/Inputs/Actions/IA_Move-RollRight.IA_Move-RollRight"))
  (bind _thruster_rollleft (Variables|Default|GetThruster_RollLeft))
  (bind _thruster_rollright (Variables|Default|GetThruster_RollRight))
  ;[1 0.3514 0 0.5] INPUTACTION: Set thurster to active and set thurster strength
  (:Triggered
    (Components|Activation|SetActive _thruster_rollright true false :!label _label)
    (Variables|/Script/Engine.PhysicsThrusterComponent|SetThrustStrength _thruster_rollright (* (* ActionValue (Variables|Default|GetThrusterPower)) 0.3))
    (Components|Activation|SetActive _thruster_rollleft true false)
    (Variables|/Script/Engine.PhysicsThrusterComponent|SetThrustStrength _thruster_rollleft (* (* (* ActionValue (Variables|Default|GetThrusterPower)) -1.0) 0.3)))
  (:Canceled
    (goto _label))
  (:Completed
    (goto _label)))

(event Input|EnhancedActionEvents|EnhancedInputActionIA_Move-RollLeft
  (params (ActionValue :type Float%20%28double-precision%29) (ElapsedSeconds :type Float%20%28double-precision%29) (TriggeredSeconds :type Float%20%28double-precision%29) (InputAction :type Input%20Action%20Object%20Reference :default "/Game/Inputs/Actions/IA_Move-RollLeft.IA_Move-RollLeft"))
  (bind _thruster_rollright (Variables|Default|GetThruster_RollRight))
  (bind _thruster_rollleft (Variables|Default|GetThruster_RollLeft))
  ;[1 0.3577 0 0.5] INPUTACTION: Set thurster to active and set thurster strength
  (:Triggered
    (Components|Activation|SetActive _thruster_rollleft true false :!label _label)
    (Variables|/Script/Engine.PhysicsThrusterComponent|SetThrustStrength _thruster_rollleft (* (* ActionValue (Variables|Default|GetThrusterPower)) 0.3))
    (Components|Activation|SetActive _thruster_rollright true false)
    (Variables|/Script/Engine.PhysicsThrusterComponent|SetThrustStrength _thruster_rollright (* (* (* ActionValue (Variables|Default|GetThrusterPower)) -1.0) 0.3)))
  (:Canceled
    (goto _label))
  (:Completed
    (goto _label)))

(event Input|EnhancedActionEvents|EnhancedInputActionIA_Shoot
  (params (ActionValue :type Boolean) (ElapsedSeconds :type Float%20%28double-precision%29) (TriggeredSeconds :type Float%20%28double-precision%29) (InputAction :type Input%20Action%20Object%20Reference :default "/Game/Inputs/Actions/IA_Shoot.IA_Shoot"))
  (bind _laserspawn (Variables|Default|GetLaserSpawn))
  ;[1 0.3398 0 0.5] INPUTACTION: SpawnActor
  (if (Variables|Default|GetCanShoot)
    (Game|SpawnActorfromClass "/Game/Blueprints/GameplayObjects/BP_LaserBlast.BP_LaserBlast_C" (Math|Transform|MakeTransform (Transformation|GetWorldLocation _laserspawn) (Transformation|GetWorldRotation _laserspawn) "5.000000,5.000000,5.000000") "AlwaysSpawn" "MultiplyWithRoot" 0 0)
    (Variables|Default|SetCurrentAmmo (Math|Integer|Clamp(Integer) (- (Variables|Default|GetCurrentAmmo) 1) 0 (Variables|Default|GetMaxAmmo)))
    (if (<= (Variables|Default|GetCurrentAmmo) 0)
      (Variables|Default|SetCanShoot false)
      (CallFunction|FReloadAmmo)
      (Utilities|FlowControl|Delay (Variables|Default|GetReloadDelay))
      (Variables|Default|SetCanShoot true)
      (else
        (Variables|Default|SetCanShoot true)))))

(event EventBeginPlay
  ;[1 0.9086 0 0.5] EVENT BeginPlay: Cast to PlayerController
  (bind _asplayer_controller (Utilities|Casting|CastToPlayerController (Pawn|GetController)))
  ;[0 0.9431 1 0.5] Checks if Input Subsystem is valid and Add the mapping context
  (Utilities|IsValid (PlayerController|LocalPlayerSubsystems|GetEnhancedInputLocalPlayerSubsystem _asplayer_controller)
    (:Is%20Valid
      (Input|AddMappingContext (PlayerController|LocalPlayerSubsystems|GetEnhancedInputLocalPlayerSubsystem _asplayer_controller) "/Game/Inputs/IMC_Astronaut.IMC_Astronaut" 0 "(bIgnoreAllPressedKeysUntilRelease=True,bForceImmediately=False,bNotifyUserSettings=False)")
      ;[0 1 0.0173 0.5] Set CurrentHealth to MaxHealth
      (Variables|Default|SetCurrentHealth (* (Variables|Default|GetMaxHealth) (Variables|Default|GetHealthUIMultiplier)))
      ;[0 1 0.0173 0.5] Set CurrentBoost to MaxBoost
      (Variables|Default|SetCurrentBoost (Variables|Default|GetMaxBoost))
      (Variables|Default|SetCurrentAmmo (Variables|Default|GetMaxAmmo))
      (Variables|Default|SetCanShoot true)
      (Audio|PlaySound2D "/Game/Assets/Sounds/space-vessel-background-noise-350616.space-vessel-background-noise-350616" 0.3 1.0 0.0 0 0))))

(event EventTick
  (params (DeltaSeconds :type Float%20%28single-precision%29))
  ;[1 0.8467 0 0.5] EVENT Tick: Call function to create a raycast
  (CallFunction|FRaycastCrosshair)
  ;[0 1 0.8738 0.5] Calculate Parallax from the Rotation and Location of the player and Reset Parallax
  (CallFunction|FCalculateParallaxfromRotation)
  (CallFunction|FResetParallax)
  (CallFunction|FCalculateParallaxfromLocation)
  (CallFunction|FResetParallax)
  (if (< (Variables|Default|GetCurrentBoost) (Variables|Default|GetMaxBoost))
    (Variables|Default|SetCurrentBoost (Math|Float|Clamp(Float) (+ (Variables|Default|GetCurrentBoost) 0.001) 0.0 (Variables|Default|GetMaxBoost)))))

(fn ConstructionScript)

(fn FRaycastCrosshair
  (bind _returnvalue (Game|GetPlayerController 0))
  (bind _laserspawn (Variables|Default|GetLaserSpawn))
  (bind _returnvalue_2 (Transformation|GetWorldLocation _laserspawn))
  ;[0 0.9235 1 0.5] Create a LineTrace
  (bind _outhit (Collision|LineTraceByChannel _returnvalue_2 (+ _returnvalue_2 (* (Math|Vector|GetForwardVector _laserspawn) (Variables|Default|GetRaycastDistance))) "TraceTypeQuery1" false 0 "None"))
  ;[0 0.9327 1 0.5] Break the hit result, set the BlockingHit and check if BlockingHit is true or false
  (bind _output_get (Variables|Default|SetBlocking%20Hit (.bBlockingHit (Collision|BreakHitResult _outhit))))
  (if _output_get
    ;[0 0.8768 1 0.5] Set ScreenPosition based on if is true or false
    (Variables|Default|SetScreen%20Position (.ScreenPosition (Class|GameplayStatics|ProjectWorldtoScreen _returnvalue (.ImpactPoint (Collision|BreakHitResult _outhit)) false)))
    (else
      (Variables|Default|SetScreen%20Position (.ScreenPosition (Class|GameplayStatics|ProjectWorldtoScreen _returnvalue (.TraceEnd (Collision|BreakHitResult _outhit)) false))))))

(fn FTakeDamage
  (params (Damage :type Integer))
  (bind _output_get (Variables|Default|SetCurrentHealth (Math|Float|Clamp(Float) (- (Variables|Default|GetCurrentHealth) (* Damage (Variables|Default|GetHealthUIMultiplier))))))
  (Development|PrintString (Utilities|String|Append "Player damaged. " "Health is: " (Utilities|String|ToString(Integer) (Class|KismetMathLibrary|ToInt64(Float) (* _output_get 1e+02)))) true true "(R=1.000000,G=0.000000,B=0.860224,A=1.000000)" 5.0))

(fn FTakeHeal
  (params (Heal :type Integer))
  (bind _output_get (Variables|Default|SetCurrentHealth (Math|Float|Clamp(Float) (+ (Variables|Default|GetCurrentHealth) (* Heal (Variables|Default|GetHealthUIMultiplier))))))
  (Development|PrintString (Utilities|String|Append "Player healed" "Health is: " (Utilities|String|ToString(Integer) (Class|KismetMathLibrary|ToInt64(Float) (* _output_get 1e+02)))) true true "(R=1.000000,G=0.000000,B=0.860224,A=1.000000)" 5.0))

(fn FCalculateParallaxfromRotation
  (bind _capsulecomponent (Variables|Collision|GetCapsuleComponent))
  (bind _minmaxpitchrate (Variables|Default|GetMinMaxPitchRate))
  (bind _minmaxyawrate (Variables|Default|GetMinMaxYawRate))
  (bind _returnvalue (Transformation|GetWorldRotation _capsulecomponent))
  (bind (_roll _pitch _yaw) (Math|Rotator|BreakRotator _returnvalue))
  (Variables|Default|SetPitchRate (Math|Float|Clamp(Float) (+ (Variables|Default|GetPitchRate) (- _pitch (.pitch (Variables|Default|GetParallaxRotator)))) (* _minmaxpitchrate -1.0) _minmaxpitchrate))
  (Variables|Default|SetYawRate (Math|Float|Clamp(Float) (+ (Variables|Default|GetYawRate) (- _yaw (.yaw (Variables|Default|GetParallaxRotator)))) (* _minmaxyawrate -1.0) _minmaxyawrate))
  (Variables|Default|SetParallaxRotator _returnvalue)
  (bind _output_get (Variables|Default|SetPitchParallaxOffset (Math|Interpolation|FInterpTo (Variables|Default|GetPitchParallaxOffset) (Variables|Default|GetPitchRate) (Utilities|Time|GetWorldDeltaSeconds) 5.0)))
  (bind _output_get_2 (Variables|Default|SetYawParallaxOffset (Math|Interpolation|FInterpTo (Variables|Default|GetYawParallaxOffset) (Variables|Default|GetYawRate) (Utilities|Time|GetWorldDeltaSeconds) 5.0)))
  (Rendering|Material|SetVectorParameterValue "/Game/Assets/Shaders/MPC_Parallax.MPC_Parallax" "ParallaxOffset" (Utilities|Struct|MakeLinearColor _output_get_2 _output_get 0.0 1.0) :!class /Script/Engine.KismetMaterialLibrary))

(fn FCalculateParallaxfromLocation
  (bind _minmaxpitchrate (Variables|Default|GetMinMaxPitchRate))
  (bind _minmaxyawrate (Variables|Default|GetMinMaxYawRate))
  (bind _capsulecomponent (Variables|Collision|GetCapsuleComponent))
  (bind _returnvalue (Transformation|GetWorldLocation _capsulecomponent))
  (bind (_x _y _z) (Math|Vector|BreakVector _returnvalue))
  (Variables|Default|SetPitchRate (Math|Float|Clamp(Float) (+ (Variables|Default|GetPitchRate) (- _x (.x (Variables|Default|GetParallaxVector)))) (* _minmaxpitchrate -1.0) _minmaxpitchrate))
  (Variables|Default|SetYawRate (Math|Float|Clamp(Float) (+ (Variables|Default|GetYawRate) (- _y (.y (Variables|Default|GetParallaxVector)))) (* _minmaxyawrate -1.0) _minmaxyawrate))
  (Variables|Default|SetParallaxVector _returnvalue)
  (bind _output_get (Variables|Default|SetPitchParallaxOffset (Math|Interpolation|FInterpTo (Variables|Default|GetPitchParallaxOffset) (Variables|Default|GetPitchRate) (Utilities|Time|GetWorldDeltaSeconds) 5.0)))
  (bind _output_get_2 (Variables|Default|SetYawParallaxOffset (Math|Interpolation|FInterpTo (Variables|Default|GetYawParallaxOffset) (Variables|Default|GetYawRate) (Utilities|Time|GetWorldDeltaSeconds) 5.0)))
  (Rendering|Material|SetVectorParameterValue "/Game/Assets/Shaders/MPC_Parallax.MPC_Parallax" "ParallaxOffset" (Utilities|Struct|MakeLinearColor _output_get_2 _output_get 0.0 1.0) :!class /Script/Engine.KismetMaterialLibrary))

(fn FResetParallax
  (Variables|Default|SetPitchRate (Math|Interpolation|FInterpTo (Variables|Default|GetPitchRate) 0.0 (Utilities|Time|GetWorldDeltaSeconds) 5.0))
  (Variables|Default|SetYawRate (Math|Interpolation|FInterpTo (Variables|Default|GetYawRate) 0.0 (Utilities|Time|GetWorldDeltaSeconds) 5.0)))

(fn FReloadAmmo
  (Variables|Default|SetCanShoot false)
  (Variables|Default|SetCurrentAmmo (Variables|Default|GetMaxAmmo))
  (Audio|PlaySound2D "/Game/Assets/Sounds/machine-gun-reload-81593.machine-gun-reload-81593" 1.0 1.0 0.0 0 0))